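; Character Blueprint that sets up default skills, server-side ability granting and AI possession.
; One tick after BeginPlay, a locally controlled character slots each DefaultSkills entry into ItemManager by array index.
; UseAIController possesses with the cached DefaultAIController, or spawns and caches one if none is valid.
; Slot-change and stat-point events are empty; gameplay-effect logic for granted effects and stat points sits disconnected.
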(event `self.ReceiveBeginPlay`
  (`parent.ReceiveBeginPlay`)
  (`KismetSystemLibrary.Delay` 0.0)
  (`self.AddDefaultSkills`))

(event `Server_GiveAbility`
  (params (AbilitySystem :type "AbilitySystemComponent Object Reference") (Ability :type "GameplayAbility Class Reference"))
  (`FPGAGameplayAbilitiesLibrary.GiveAbility` AbilitySystem Ability))

(event `UseAIController`
  (`self.DefaultAIController`
    (:`then`
      (`Controller.Possess` (`self.DefaultAIController`) self))
    (:`else`
      (`self.SpawnDefaultController`)
      (bind _asaicontroller (cast `AIController` (`self.GetController`)))
      ;[1 0 0.1406] TODO Turn on RVO avoidance
      (set `self.DefaultAIController` _asaicontroller))))

(event `self.ItemManager.OnSlottedItemChanged`
  (params (ItemSlot :type "FPGAItemSlot Structure") (Item :type "FPGABaseItem Object Reference")))

(event `ApplyStatPoints`
  (params (Attribute :type "GameplayAttribute Structure") (Amount :type Integer :default 1)))

(fn `AddDefaultSkills`
  (if (`self.IsLocallyControlled`)
    (for (_array_element _array_index) (`self.DefaultSkills`)
      (`FPGAItemManager.SetSlottedItem` (`self.ItemManager`) (make `FPGAItemSlot` "Skill" _array_index) _array_element true))))

(fn `UserConstructionScript`)