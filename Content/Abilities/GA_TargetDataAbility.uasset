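; Base targeted gameplay ability that acquires target data, then offers a move-to-and-attack montage loop for child abilities.
; Players target through a cursor target actor, applying block/cancel tags; AI-controlled pawns use GetTargetDataFromAI, an empty stub here.
; MoveToAndPlayAnimation moves and faces within range, plays the montage unless blocking tags exist, forwards notifies, and repeats unless end flags are set.
; The ability ends when the target actor gains the death tag.
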(event `MoveToAndPlayAnimation`
  (params (MontageToPlay :type "AnimMontage Object Reference") (MontageTaskName :type Name :default "CastMontage") (MaxRange :type "Float (double-precision)" :default 500.0))
  (`KismetSystemLibrary.PrintString` "Move and play anim")
  (bind _asynctaskproxy (`FPGAAbilityTask_SimpleMoveAndFace.SimpleMoveAndFace` "MovementTask" MaxRange (0.0 0.0 0.0) (`|GetArrayItem` (`AbilitySystemBlueprintLibrary.GetAllActorsFromTargetData` (`self.TargetData`))) false :!label _label)
    (:`then`
      (set `self.MovementTask` _asynctaskproxy))
    (:`OnFinish`
      (bind _returnvalue (`self.CanPlayMontage`))
      (if _returnvalue
        (bind _movementtask (`self.MovementTask`)
          (:`then`
            (`GameplayTask.EndTask` _movementtask)
            (`KismetSystemLibrary.PrintString` "ATTACK MONT")
            (bind (_asynctaskproxy_2 _notifyname) (`FPGAAbilityTask_PlayMontageNotify.CreatePlayMontageAndWaitProxy` MontageTaskName MontageToPlay (`self.GetMontageTime`))
              (:`OnCompleted`
                (if (`self.bEndOnMontageCompleted`)
                  (`self.K2_EndAbility` :!label _label_2)
                  (else
                    (goto _label))))
              (:`OnInterrupted`
                (if (`self.bEndOnInterrupt`)
                  (goto _label_2)
                  (else
                    (`KismetSystemLibrary.PrintString` "Intterupt")
                    (goto _label))))
              (:`OnCancelled`
                (goto _label_2))
              (:`OnNotifyBegin`
                (`self.OnMontageNotify` _notifyname))
              (:`OnCancel`
                (goto _label_2))))
          (:`else`))))
    (:`OnCancel`
      (`self.K2_EndAbility`))))

(event `self.K2_ActivateAbility`
  (`parent.K2_ActivateAbility`)
  (`self.SetTargetData`))

(event `SetTargetData`
  (`/Engine/EditorBlueprintResources/StandardMacros.IsValid` (`.PlayerController` (break `GameplayAbilityActorInfo` (`self.GetActorInfo`)))
    (:`Is Valid`
      (bind (_asynctaskproxy _data) (`FPGAAbilityTask_WaitTargetData.FPGAWaitTargetData` "None" (`self.ConfirmationType`) "/Script/FPGameplayAbilities.FPGATargetActor_Cursor" (`self.TargetType`) (`self.ObjectTypes`) (struct) (struct) null (`self.Filter`))
        (:`ValidData`
          (set `self.TargetData` _data)
          (`FPGAGameplayAbilitiesLibrary.BlockAbilitiesWithTags` (`self.GetAbilitySystemComponentFromActorInfo`) (`self.BlockAbilitiesWithTagsOnSetTargetData`))
          (`FPGAGameplayAbilitiesLibrary.CancelAbilitiesWithTags` (`self.GetAbilitySystemComponentFromActorInfo`) self (`self.CancelAbilitiesWithTagsOnSetTargetData`))
          (`self.BindTargetActorDeath`)
          (`self.OnSetTargetData`))
        (:`Cancelled`
          (`self.K2_EndAbility`))))
    (:`Is Not Valid`
      (bind _aspawn (cast `Pawn` (`.OwnerActor` (break `GameplayAbilityActorInfo` (`self.GetActorInfo`))))
        (:`then`
          (bind _asaicontroller (cast `AIController` (`Pawn.GetController` _aspawn))
            (:`then`
              (bind _targetdata (`self.GetTargetDataFromAI` _asaicontroller))
              (set `self.TargetData` _targetdata)
              (`self.BindTargetActorDeath`)
              (`self.OnSetTargetData`))
            (:`CastFailed`
              (`self.K2_EndAbility` :!label _label_3))))
        (:`CastFailed`
          (goto _label_3))))))

(event `self.K2_OnEndAbility`
  (params (bWasCancelled :type Boolean))
  (`parent.K2_OnEndAbility` bWasCancelled)
  (`FPGAGameplayAbilitiesLibrary.UnBlockAbilitiesWithTags` (`self.GetAbilitySystemComponentFromActorInfo`) (`self.BlockAbilitiesWithTagsOnSetTargetData`)))

(event `OnSetTargetData`)

(event `BindTargetActorDeath`
  (bind _targetdata (`self.TargetData`))
  (if (`AbilitySystemBlueprintLibrary.TargetDataHasActor` _targetdata)
    (`AbilityTask_WaitGameplayTagAdded.WaitGameplayTagAdd` (struct :`TagName` "Status.Debuff.Strong.Death") (`|GetArrayItem` (`AbilitySystemBlueprintLibrary.GetAllActorsFromTargetData` _targetdata))
      (:`Added`
        (`self.K2_EndAbility`)))))

(fn `CanPlayMontage`
  (returns (ReturnValue :type Boolean))
  (bind _returnvalue (message `GameplayTagAssetInterface.HasAnyMatchingGameplayTags` (`self.GetAbilitySystemComponentFromActorInfo`) (`self.MontageBlockingTags`)))
  (return (not _returnvalue)))

(fn `GetMontageTime`
  (returns (ReturnValue :type "Float (double-precision)"))
  (return (`self.AnimationTime`)))

(fn `GetTargetDataFromAI`
  (params (AIController :type "AIController Object Reference"))
  (returns (TargetData :type "GameplayAbilityTargetDataHandle Structure"))
  (return))