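; GA_FPGAAbility is a Gameplay Ability that appears to serve as a base, providing debuff handling, montage playback and cost/cooldown setup.
; On activation it watches CannotMove, CannotAttack and CannotCast tags, ending named movement or montage tasks and firing empty hook events, including on CannotMove removal.
; SimplePlayMontage forwards notifies and ends the ability when playback finishes or breaks off.
; Mana cost and cooldown use SetByCaller magnitudes; cooldown is also debug-printed.
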(event `self.K2_ActivateAbility`
  (`|ExecutionSequence`
    (:`then_0`
      (`AbilityTask_WaitGameplayTagAdded.WaitGameplayTagAdd` (struct :`TagName` "Status.Debuff.Weak.CannotMove") null
        (:`then`
          (`AbilityTask_WaitGameplayTagAdded.WaitGameplayTagAdd` (struct :`TagName` "Status.Debuff.Weak.CannotAttack") null
            (:`then`
              (`AbilityTask_WaitGameplayTagAdded.WaitGameplayTagAdd` (struct :`TagName` "Status.Debuff.Weak.CannotCast") null
                (:`Added`
                  (`self.EndTaskByInstanceName` "CastMontage")
                  (`self.OnCannotCastTag`))))
            (:`Added`
              (`self.EndTaskByInstanceName` "AttackMontage")
              (`self.OnCannotAttackTag`))))
        (:`Added`
          (`self.EndTaskByInstanceName` "MovementTask")
          (`self.OnCannotMoveTag`))))
    (:`then_1`
      (`AbilityTask_WaitGameplayTagRemoved.WaitGameplayTagRemove` (struct :`TagName` "Status.Debuff.Weak.CannotMove") null
        (:`Removed`
          (`self.OnCannotMoveTagRemoved`))))))

(event `SimplePlayMontage`
  (params (MontageToPlay :type "AnimMontage Object Reference") (MontageTaskName :type Name :default "CastAnimation"))
  (bind (_asynctaskproxy _notifyname) (`FPGAAbilityTask_PlayMontageNotify.CreatePlayMontageAndWaitProxy` MontageTaskName MontageToPlay)
    (:`OnCompleted`
      (`self.K2_EndAbility` :!label _label))
    (:`OnInterrupted`
      (goto _label))
    (:`OnCancelled`
      (goto _label))
    (:`OnNotifyBegin`
      (`self.OnMontageNotify` _notifyname))
    (:`OnCancel`
      (goto _label))))

(event `OnMontageNotify`
  (params (NotifyName :type Name)))

(event `OnCannotMoveTag`)

(event `OnCannotMoveTagRemoved`)

(event `OnCannotAttackTag`)

(event `OnCannotCastTag`)

(fn `AdjustCooldownSpec`
  (params (CooldownSpec :type "GameplayEffectSpec Structure (by ref)"))
  (bind _cooldown (`self.Cooldown`))
  (`KismetSystemLibrary.PrintString` (`KismetStringLibrary.Conv_DoubleToString` _cooldown))
  (`FPGAGameplayAbilitiesLibrary.SetSetByCallerMagnitude` CooldownSpec (struct :`TagName` "Mag.Cooldown") _cooldown)
  (return))

(fn `AdjustCostSpec`
  (params (CostSpec :type "GameplayEffectSpec Structure (by ref)"))
  (`FPGAGameplayAbilitiesLibrary.SetSetByCallerMagnitude` CostSpec (struct :`TagName` "Mag.Cost.Mana") (* (`self.ManaCost`) -1.0))
  (return))