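; Game mode that announces each new player login to the FPGA player controllers on the server.
; On PostLogin it waits briefly, then prints a join message with the new player's ID.
; It then loops over player indices, casts each controller to BP_FPGAPlayerController and calls OnPlayerJoined on it, which includes the newcomer as well as existing players.
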(event `self.K2_PostLogin`
  (params (NewPlayer :type "PlayerController Object Reference"))
  (`KismetSystemLibrary.Delay` 0.25)
  (`KismetSystemLibrary.PrintString` (`KismetStringLibrary.Concat_StrStr` "Player Joined " (`KismetStringLibrary.Conv_IntToString` (`PlayerState.PlayerId` (`Controller.PlayerState` NewPlayer)))))
  (for _index (range (`self.NumPlayers`))
    (bind _asbp_fpgaplayer_controller (cast `/FPGameplayAbilities/BP_FPGAPlayerController` (`GameplayStatics.GetPlayerController` _index)))
    (`/FPGameplayAbilities/BP_FPGAPlayerController.OnPlayerJoined` _asbp_fpgaplayer_controller)))

(fn `UserConstructionScript`)