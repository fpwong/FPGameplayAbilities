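; BP_FPGAAOEReticle is a Gameplay Ability targeting reticle that shows an area of effect with a decal.
; The construction script creates a dynamic material instance on the decal, and parameter initialization feeds the X of the AOE scale into its Radius parameter.
; The reticle is hidden whenever the target is invalid.
; Disconnected leftover nodes for actor scaling, Niagara radius and debug printing never run.
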(event `self.OnParametersInitialized`
  (`MaterialInstanceDynamic.SetScalarParameterValue` (`self.MaterialInstance`) "Radius" (.x (`.AOEScale` (break `WorldReticleParameters` (`self.Parameters`))))))

(event `self.OnValidTargetChanged`
  (params (bNewValue :type Boolean))
  (`self.SetActorHiddenInGame` (not bNewValue)))

(fn `UserConstructionScript`
  (bind _returnvalue (`DecalComponent.CreateDynamicMaterialInstance` (`self.Decal`)))
  (set `self.MaterialInstance` _returnvalue))