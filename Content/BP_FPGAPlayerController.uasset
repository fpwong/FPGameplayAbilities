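; Player controller that turns five skill inputs into Gameplay Ability activations and supports switching between unclaimed pawns.
; Each input activates the first ability granted by the matching FPGAItemManager slot, playing a sound on failure.
; Server possession hands the previous character back to AI, while the owner waits for a valid pawn before binding a still-empty slot-change handler.
; Remote instances simulate packet lag on BeginPlay, and the cursor-pick possession logic is disconnected.
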(event `self.ReceiveBeginPlay`
  (`/Engine/EditorBlueprintResources/ActorMacros.Switch Has Authority`
    (:`Remote`
      (`KismetSystemLibrary.Delay` 0.2)
      (`KismetSystemLibrary.ExecuteConsoleCommand` "Net PktLag=125" null))))

(event `OnPlayerJoined`
  ;[1 0.9375 0] On player joined
)

(event `ActivateSkill`
  (params (SkillSlot :type Integer))
  (bind _returnvalue (`FPGAItemManager.GetSlottedItem` (`self.GetComponentByClass` (`self.K2_GetPawn`) "/Script/FPGameplayAbilities.FPGAItemManager") (make `FPGAItemSlot` "Skill" SkillSlot)))
  (bind _grantedabilities (`FPGABaseItem.GrantedAbilities` _returnvalue))
  (bind _output (`|GetArrayItem` _grantedabilities))
  (`/Engine/EditorBlueprintResources/StandardMacros.IsValid` _returnvalue
    (:`Is Valid`
      (if (`KismetArrayLibrary.Array_IsValidIndex` _grantedabilities)
        (`KismetSystemLibrary.PrintString` (`KismetSystemLibrary.GetClassDisplayName` _output))
        (bind _returnvalue_2 (`AbilitySystemComponent.TryActivateAbilityByClass` (`AbilitySystemBlueprintLibrary.GetAbilitySystemComponent` (`self.K2_GetPawn`)) _output true))
        (if (not _returnvalue_2)
          (`GameplayStatics.PlaySound2D` "/Engine/VREditor/Sounds/UI/Camera_Shutter.Camera_Shutter" 1.0 1.0 0.0 null null))))))

(event `InputAction|Skill_1`
  (params (Key :type "Key Structure"))
  ;[1 0 0.2109] Skill input and activation
  (:`Pressed`
    (`self.ActivateSkill` 0)))

(event `InputAction|Skill_2`
  (params (Key :type "Key Structure"))
  ;[1 0 0.2109] Skill input and activation
  (:`Pressed`
    (`self.ActivateSkill` 1)))

(event `InputAction|Skill_3`
  (params (Key :type "Key Structure"))
  ;[1 0 0.2109] Skill input and activation
  (:`Pressed`
    (`self.ActivateSkill` 2)))

(event `InputAction|Skill_4`
  (params (Key :type "Key Structure"))
  ;[1 0 0.2109] Skill input and activation
  (:`Pressed`
    (`self.ActivateSkill` 3)))

(event `InputAction|Skill_5`
  (params (Key :type "Key Structure"))
  (:`Pressed`
    (`self.ActivateSkill` 4)))

(event `self.ReceivePossess`
  (params (PossessedPawn :type "Pawn Object Reference"))
  (`parent.ReceivePossess` PossessedPawn)
  (`KismetSystemLibrary.PrintString` (`KismetSystemLibrary.GetDisplayName` PossessedPawn))
  (`self.Owning_OnPossess`))

(event `Owning_OnPossess`
  (`/Engine/EditorBlueprintResources/StandardMacros.IsValid` (`self.K2_GetPawn`) :!label _label
    (:`Is Valid`
      (`KismetSystemLibrary.Delay` 0.0 :!pinned true) ; Delay 1 frame for pawn to init
      (`self.OnPossessAndValidPawn`))
    (:`Is Not Valid`
      (`KismetSystemLibrary.Delay` 0.1)
      (goto _label))))

(event `OnPossessAndValidPawn`
  (add `FPGAItemManager.OnSlottedItemChanged` (`self.GetComponentByClass` (`self.K2_GetPawn`) "/Script/FPGameplayAbilities.FPGAItemManager") (delegate `OnSlottedItemChanged`)))

(event `OnSlottedItemChanged`
  (params (ItemSlot :type "FPGAItemSlot Structure") (Item :type "FPGABaseItem Object Reference")))

(event `Server_Possess`
  (params (InPawn :type "Pawn Object Reference"))
  (bind _returnvalue (`self.K2_GetPawn`))
  (cast `PlayerController` (`Pawn.GetController` InPawn)
    (:`CastFailed`
      (`|ExecutionSequence`
        (:`then_0`
          (`/Engine/EditorBlueprintResources/StandardMacros.IsValid` _returnvalue
            (:`Is Valid`
              (set `self.PreviouslyControlledPawn` _returnvalue))))
        (:`then_1`
          (`self.Possess` InPawn))
        (:`then_2`
          (bind _asbp_fpgacharacter (cast `/FPGameplayAbilities/BP_FPGACharacter` (`self.PreviouslyControlledPawn`)))
          (`/FPGameplayAbilities/BP_FPGACharacter.UseAIController` _asbp_fpgacharacter))))))

(fn `UserConstructionScript`)