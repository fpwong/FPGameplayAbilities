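; BP_GroundEffect is a ground area actor that keeps a burn debuff on actors inside its sphere.
; Overlap begin applies GE_Debuff_Burn through the entering actor's own Ability System Component, and overlap end removes all stacks of it.
; BeginPlay registers and activates the sphere with FPCHitboxHelper, but that helper's overlap event is empty, so the sphere's component overlaps drive the effect.
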(event `self.ReceiveBeginPlay`
  (bind _fpchitboxhelper (`self.FPCHitboxHelper`))
  (`FPCHitboxHelper.RegisterHitbox` _fpchitboxhelper (`self.Sphere`) 0)
  (`FPCHitbox.SetHitboxActive` (`FPCHitboxHelper.GetHitbox` _fpchitboxhelper 0) true))

(event `self.FPCHitboxHelper.OnHitboxOverlap`
  (params (Actor :type "Actor Object Reference") (Hitbox :type "FPCHitbox Object Reference") (HitboxHelper :type "FPCHitboxHelper Object Reference") (Hit :type "HitResult Structure (by ref)")))

(event `self.Sphere.OnComponentBeginOverlap`
  (params (OverlappedComponent :type "PrimitiveComponent Object Reference") (OtherActor :type "Actor Object Reference") (OtherComp :type "PrimitiveComponent Object Reference") (OtherBodyIndex :type Integer) (bFromSweep :type Boolean) (SweepResult :type "HitResult Structure (by ref)"))
  (bind _returnvalue (`AbilitySystemBlueprintLibrary.GetAbilitySystemComponent` OtherActor))
  (`/Engine/EditorBlueprintResources/StandardMacros.IsValid` _returnvalue
    (:`Is Valid`
      (`AbilitySystemComponent.BP_ApplyGameplayEffectToTarget` :`self` _returnvalue :`GameplayEffectClass` "/Game/CoopRPG/Characters/Healer/Bubble/GE_Debuff_Burn.GE_Debuff_Burn_C" :`Target` _returnvalue))))

(event `self.Sphere.OnComponentEndOverlap`
  (params (OverlappedComponent :type "PrimitiveComponent Object Reference") (OtherActor :type "Actor Object Reference") (OtherComp :type "PrimitiveComponent Object Reference") (OtherBodyIndex :type Integer))
  (bind _returnvalue (`AbilitySystemBlueprintLibrary.GetAbilitySystemComponent` OtherActor))
  (`/Engine/EditorBlueprintResources/StandardMacros.IsValid` _returnvalue
    (:`Is Valid`
      (`AbilitySystemComponent.RemoveActiveGameplayEffectBySourceEffect` _returnvalue "/Game/CoopRPG/Characters/Healer/Bubble/GE_Debuff_Burn.GE_Debuff_Burn_C" null -1))))

(fn `UserConstructionScript`)